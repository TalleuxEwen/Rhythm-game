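; Title screen Blueprint that shows the title and currently-playing widgets on BeginPlay, with UI-only input and a visible cursor.
; It also imports WAV files from a path through Runtime Audio Importer.
; On a successful import, the result callback passes the sound wave to Editor widgets found in the viewport.
; Direct 2D playback is disconnected, and a separate OnPrepared handler plays the audio component but is not bound here.
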(event `self.ReceiveBeginPlay`
  (bind _returnvalue (`GameplayStatics.GetPlayerController` 0))
  (bind _returnvalue_2 (`|CreateWidget` "/Game/UITemplate/Widgets/WBP_TitleScreen.WBP_TitleScreen_C" _returnvalue))
  (`UserWidget.AddToViewport` _returnvalue_2 0)
  (`WidgetBlueprintLibrary.SetInputMode_UIOnlyEx` _returnvalue null)
  (set `PlayerController.bShowMouseCursor` true _returnvalue)
  (bind _returnvalue_3 (`|CreateWidget` "/Game/Blueprints/Widgets/WBP_CurrentlyPlaying.WBP_CurrentlyPlaying_C" (`GameplayStatics.GetPlayerController` 0)))
  (`UserWidget.AddToViewport` _returnvalue_3 0))

(fn `BP_EditorView_AutoGenFunc`
  (params (bSucceeded :type Boolean) (AudioData :type "Array of Byte (by ref)"))
  (for _index (range (+ (`KismetArrayLibrary.Array_Length` AudioData) 1))
    _))

(fn `OnPrepared`
  (params (bSucceeded :type Boolean))
  (if bSucceeded
    (`AudioComponent.SetWaveParameter` (`self.Audio Component`) "Name" (`self.Imported Sound Wave`))
    (`KismetSystemLibrary.PrintString` "Hello")
    (`AudioComponent.Play` (`self.Audio Component`) 0.0)
    (else
      (`KismetSystemLibrary.PrintString` "Marche po"))))

(fn `OnResult`
  (params (Importer :type "RuntimeAudioImporterLibrary Object Reference") (ImportedSoundWave :type "ImportedSoundWave Object Reference") (Status :type "ERuntimeImportStatus Enum" :default "SuccessfulImport"))
  (switch `ERuntimeImportStatus` Status
    (:`SuccessfulImport`
      (bind _foundwidgets (`WidgetBlueprintLibrary.GetAllWidgetsOfClass` "/Game/Editor/Editor.Editor_C"))
      (`/Game/Editor/Editor.SetAudioComponent` _foundwidgets ImportedSoundWave))))

(fn `OpenAndPlayWavFile`
  (params (FilePath :type String))
  (bind _returnvalue (`RuntimeAudioImporterLibrary.CreateRuntimeAudioImporter`))
  (bind _output_get (set `self.Audio Importer` _returnvalue))
  (add `RuntimeAudioImporterLibrary.OnResult` _output_get (`|CreateDelegate` :!event `OnResult`))
  (bind _returnvalue_2 (`AddComponent|NODE_AddAudioComponent-2`))
  (set `self.Audio Component` _returnvalue_2)
  (`RuntimeAudioImporterLibrary.ImportAudioFromFile` (`self.Audio Importer`) FilePath "Wav"))

(fn `UserConstructionScript`)