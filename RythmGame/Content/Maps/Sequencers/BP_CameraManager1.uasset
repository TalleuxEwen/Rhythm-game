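; Camera manager Blueprint that plays random level sequences from SequenceArray back to back, starting on BeginPlay.
; Each sequence gets a newly created player whose OnFinished event triggers PLayNewSequencer to start the next.
; GetRandomInt attempts to avoid repeating the current index through recursion, but its separate random rolls and discarded recursive result do not guarantee a different one.
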(event `self.ReceiveBeginPlay`
  (bind _sequencearray (`self.SequenceArray`))
  (bind _output_get (set `self.RandInt` (`KismetMathLibrary.RandomInteger` (`KismetArrayLibrary.Array_Length` _sequencearray))))
  (bind (_outactor _returnvalue) (`LevelSequencePlayer.CreateLevelSequencePlayer` (`|GetArrayItem` _sequencearray _output_get)))
  (`MovieSceneSequencePlayer.Play` _returnvalue)
  (add `MovieSceneSequencePlayer.OnFinished` _returnvalue (delegate `PLayNewSequencer`)))

(event `PLayNewSequencer`
  (bind _randint (`self.GetRandomInt`))
  (bind _output_get (set `self.RandInt` _randint))
  (bind (_outactor _returnvalue) (`LevelSequencePlayer.CreateLevelSequencePlayer` (`|GetArrayItem` (`self.SequenceArray`) _output_get)))
  (`MovieSceneSequencePlayer.Play` _returnvalue)
  (add `MovieSceneSequencePlayer.OnFinished` _returnvalue (delegate `PLayNewSequencer`)))

(fn `GetRandomInt`
  (returns (RandInt :type Integer))
  (bind _returnvalue (`KismetMathLibrary.RandomInteger` (`KismetArrayLibrary.Array_Length` (`self.SequenceArray`))))
  (if (== (`self.RandInt`) _returnvalue)
    (`self.GetRandomInt`)
    (else
      (return _returnvalue))))

(fn `UserConstructionScript`)