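; BP_MapPlayer runs a lane-based rhythm game map, setting up the HUD, six child lane actors and key-press lane animations.
; It takes notes and key count from BP_Maploader and song data from GI_Music, shifting and hiding lanes to suit.
; A BPM timer spawns spheres from six-slot rows of the flat note array.
; A lane event starts MetaSound playback; audio stopping, or never starting, opens the score-saving end screen.
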(event `self.ReceiveBeginPlay`
  (bind _returnvalue (`|CreateWidget` "/Game/Game/Blueprints/Widgets/WBP_HUD.WBP_HUD_C"))
  (bind _returnvalue_2 (`|CreateWidget` "/Game/Editor/Blueprints/WBP_LoadingForMetaSound.WBP_LoadingForMetaSound_C"))
  (`UserWidget.AddToViewport` _returnvalue_2 0)
  (`UserWidget.AddToViewport` _returnvalue 0)
  (bind _asbp_player (cast `/Game/Game/Blueprints/BP_Player` (`GameplayStatics.GetPlayerCharacter` 0)))
  (add `/Game/Game/Blueprints/BP_Player.KeyPress` _asbp_player (delegate `KeyPressed`))
  (`self.SetupSceneMap`)
  (bind _returnvalue_3 (`GameplayStatics.GetActorOfClass` "/Game/Game/Blueprints/BP_Maploader.BP_Maploader_C"))
  (bind (_notearray _nbkeys) (`/Game/Game/Blueprints/BP_Maploader.LoadMap` _returnvalue_3))
  (set `self.Note Array` _notearray)
  (set `self.Nb Keys` _nbkeys)
  (`self.HandleNbKeys`)
  (bind _asgi_music (cast `/Game/Blueprints/GI_Music` (`GameplayStatics.GetGameInstance`)))
  (set `self.BPM` (`/Game/Blueprints/GI_Music.BPM` _asgi_music))
  (set `self.Offset` (`/Game/Blueprints/GI_Music.Offset` _asgi_music))
  (set `self.Song Name` (`/Game/Blueprints/GI_Music.SongName` _asgi_music))
  (set `self.File Name` (`/Game/Blueprints/GI_Music.FileName` _asgi_music))
  (set `self.Imported Sound Wave` (`/Game/Blueprints/GI_Music.AudioComponent` _asgi_music))
  (bind _returnvalue_4 (`AddComponent|NODE_AddAudioComponent-0`))
  (set `self.AudioComponent` _returnvalue_4)
  (`Widget.RemoveFromParent` _returnvalue_2)
  (`self.StartPlayingMap`)
  (bind _outactors (`GameplayStatics.GetAllActorsOfClass` "/Game/Game/Blueprints/BP_SingleLane.BP_SingleLane_C"))
  (for _array_element _outactors
    (add `/Game/Game/Blueprints/BP_SingleLane.TriggerMusicPlay` _array_element (delegate `CustomEvent_0`)))
  (`KismetSystemLibrary.Delay` 10.0)
  (if (not (`self.MusicTriggered`))
    (bind _foundwidgets (`WidgetBlueprintLibrary.GetAllWidgetsOfClass` "/Game/Editor/Blueprints/WBP_EndGame.WBP_EndGame_C" :!label _label))
    (if (not (`KismetMathLibrary.Conv_IntToBool` (`KismetArrayLibrary.Array_Length` _foundwidgets)))
      (`self.EndGame`))))

(event `CustomEvent_0`
  (bind _musictriggered (`self.MusicTriggered`))
  (`KismetSystemLibrary.PrintString` (`KismetStringLibrary.Conv_BoolToString` _musictriggered))
  (if (not _musictriggered)
    (`self.PlayInMetaSound` (`self.Imported Sound Wave`))
    (set `self.MusicTriggered` true)))

(event `KeyPressed`
  (params (KeyNumber :type Integer))
  (`/Game/Game/Blueprints/BP_SingleLane.StartAnimation` (`BlueprintMapLibrary.Map_Find` (`self.SceneMap`) KeyNumber)))

(event `StartPlayingMap`
  (`KismetSystemLibrary.Delay` 3.0)
  (`KismetSystemLibrary.K2_SetTimerDelegate` (delegate `PlayNotes`) (/ 60.0 (`self.BPM`)) true))

(event `PlayNotes`
  (bind _note_array (`self.Note Array`))
  (if (`self.MusicTriggered`)
    (if (`|EnumEquality` (`AudioComponent.GetPlayState` (`self.AudioComponent`)) "Stopped")
      (goto _label)
      (else
        _)))
  (for _index (range 6)
    (bind _returnvalue (+ (`self.CurrentNoteInArray`) _index))
    (if (< _returnvalue (`KismetArrayLibrary.Array_Length` _note_array))
      (if (`|GetArrayItem` _note_array _returnvalue)
        (`/Game/Game/Blueprints/BP_SingleLane.SpawnSphere` (`BlueprintMapLibrary.Map_Find` (`self.SceneMap`) (+ _index 1)) (`self.BPM`)))))
  (bind _output_get (set `self.CurrentNoteInArray` (+ (`self.CurrentNoteInArray`) 6))))

(fn `EndGame`
  (bind _returnvalue (`GameplayStatics.GetPlayerController` 0))
  (bind _returnvalue_2 (`|CreateWidget` "/Game/Editor/Blueprints/WBP_EndGame.WBP_EndGame_C"))
  (`UserWidget.AddToViewport` _returnvalue_2 3)
  (bind _foundwidgets (`WidgetBlueprintLibrary.GetAllWidgetsOfClass` "/Game/Game/Blueprints/Widgets/WBP_HUD.WBP_HUD_C"))
  (set `/Game/Editor/Blueprints/WBP_EndGame.score` (`/Game/Game/Blueprints/Widgets/WBP_HUD.Score` (`|GetArrayItem` _foundwidgets)) _returnvalue_2)
  (`/Game/Editor/Blueprints/WBP_EndGame.SaveHighScore` _returnvalue_2 (`self.File Name`))
  (`WidgetBlueprintLibrary.SetInputMode_UIOnlyEx` _returnvalue null)
  (set `PlayerController.bShowMouseCursor` true _returnvalue))

(fn `HandleNbKeys`
  (if (!= (`self.Nb Keys`) 6)
    (for _index (range 1 (+ (`self.Nb Keys`) 1))
      (`self.K2_AddActorWorldOffset` (`BlueprintMapLibrary.Map_Find` (`self.SceneMap`) _index) (`KismetMathLibrary.MakeVector` (`KismetMathLibrary.Conv_IntToDouble` (* (- 6 (`self.Nb Keys`)) 85))) false false))
    (if (< (`self.Nb Keys`) 6)
      (for _index_2 (range (+ (`self.Nb Keys`) 1) 7)
        (`self.SetActorHiddenInGame` (`BlueprintMapLibrary.Map_Find` (`self.SceneMap`) _index_2) true)))))

(fn `PlayInMetaSound`
  (params (InWave :type "SoundWave Object Reference") (NewParam :type Boolean))
  (`AudioComponent.SetWaveParameter` (`self.AudioComponent`) "ImportedWave" InWave)
  (`AudioComponent.SetFloatParameter` (`self.AudioComponent`) "Start Timeeee" (`self.Offset`))
  (`AudioComponent.Play` (`self.AudioComponent`) 0.0))

(fn `SetupSceneMap`
  (bind _asbp_single_lane (cast `/Game/Game/Blueprints/BP_SingleLane` (`ChildActorComponent.ChildActor` (`self.BP_SingleLane1`))))
  (`BlueprintMapLibrary.Map_Add` (`self.SceneMap`) 1 _asbp_single_lane)
  (bind _asbp_single_lane_2 (cast `/Game/Game/Blueprints/BP_SingleLane` (`ChildActorComponent.ChildActor` (`self.BP_SingleLane2`))))
  (`BlueprintMapLibrary.Map_Add` (`self.SceneMap`) 2 _asbp_single_lane_2)
  (bind _asbp_single_lane_3 (cast `/Game/Game/Blueprints/BP_SingleLane` (`ChildActorComponent.ChildActor` (`self.BP_SingleLane3`))))
  (`BlueprintMapLibrary.Map_Add` (`self.SceneMap`) 3 _asbp_single_lane_3)
  (bind _asbp_single_lane_4 (cast `/Game/Game/Blueprints/BP_SingleLane` (`ChildActorComponent.ChildActor` (`self.BP_SingleLane4`))))
  (`BlueprintMapLibrary.Map_Add` (`self.SceneMap`) 4 _asbp_single_lane_4)
  (bind _asbp_single_lane_5 (cast `/Game/Game/Blueprints/BP_SingleLane` (`ChildActorComponent.ChildActor` (`self.BP_SingleLane5`))))
  (`BlueprintMapLibrary.Map_Add` (`self.SceneMap`) 5 _asbp_single_lane_5)
  (bind _asbp_single_lane_6 (cast `/Game/Game/Blueprints/BP_SingleLane` (`ChildActorComponent.ChildActor` (`self.BP_SingleLane6`))))
  (`BlueprintMapLibrary.Map_Add` (`self.SceneMap`) 6 _asbp_single_lane_6))

(fn `UserConstructionScript`)