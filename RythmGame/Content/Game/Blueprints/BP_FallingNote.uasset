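; BP_FallingNote is a note actor, apparently for a rhythm game, that moves its Sphere along a falling path and destroys itself when Hit.
; StartFalling runs two chained timelines: the first lerps from start to end location, the second continues to the full end location.
; Both scale the timeline value by half the BPM to form the lerp alpha, so tempo sets travel speed.
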(event `StartFalling`
  (params (StartLocation :type "Vector Structure") (EndLocation :type "Vector Structure") (FullEndLocation :type "Vector Structure") (BPM :type "Float (double-precision)" :default 1.0))
  (bind _returnvalue (/ BPM 2.0))
  (bind (_direction _newtrack_0) (`Timeline|Timeline` :!via `PlayFromStart`)
    (:`Update`
      (`SceneComponent.K2_SetWorldLocation` (`self.Sphere`) (`KismetMathLibrary.VLerp` StartLocation EndLocation (* _newtrack_0 _returnvalue)) false false))
    (:`Finished`
      (bind (_direction_2 _newtrack_0_2) (`Timeline|Timeline_0` :!via `PlayFromStart`)
        (:`Update`
          (`SceneComponent.K2_SetWorldLocation` (`self.Sphere`) (`KismetMathLibrary.VLerp` EndLocation FullEndLocation (* _newtrack_0_2 _returnvalue)) false false))))))

(event `/Game/Game/Blueprints/BPI_HitObject.Hit`
  (`self.K2_DestroyActor`))

(fn `UserConstructionScript`)