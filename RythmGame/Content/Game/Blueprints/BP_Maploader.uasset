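; BP_Maploader loads a note map for a music game from a text file.
; LoadMap takes the file name from GI_Music, runs ParseGameData and returns the note array and key count, printing a message if no name is set.
; ParseGameData reads lines through FileSDK, takes the key count from the "NbKeys:" header, then flattens each following line's true/false tokens into one boolean NoteArray.
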(fn `LoadMap`
  (returns (NoteArray :type "Array of Boolean") (NbKeys :type Integer))
  (bind _asgi_music (cast `/Game/Blueprints/GI_Music` (`GameplayStatics.GetGameInstance`)))
  (bind _filename (`/Game/Blueprints/GI_Music.FileName` _asgi_music))
  (if (`KismetStringLibrary.IsEmpty` _filename)
    (`KismetSystemLibrary.PrintString` "No filename set" true true (struct :`R` 1.0 :`B` 0.032032 :`A` 1.0))
    (return (`self.NoteArray`) (`self.NbKeys`))
    (else
      (`self.ParseGameData` _filename)
      (return (`self.NoteArray`) (`self.NbKeys`)))))

(fn `ParseGameData`
  (params (FileName :type String))
  (locals (StartParsing :type Boolean))
  (for _array_element (`FileSDKBPLibrary.ReadLinesFromFile` FileName "/Script/FileSDK.FileSDKLineReader")
    (if (`local.StartParsing`)
      (for _array_element_2 (`KismetStringLibrary.ParseIntoArray` _array_element)
        (`KismetArrayLibrary.Array_Add` (`self.NoteArray`) (== _array_element_2 "true")))
      (else
        (bind _returnvalue (`KismetStringLibrary.ReplaceInline` _array_element "NbKeys:"))
        (if (`KismetMathLibrary.Conv_IntToBool` _returnvalue)
          (set `self.NbKeys` (`KismetStringLibrary.Conv_StringToInt` (`KismetStringLibrary.Replace` _array_element "NbKeys:")))
          (set `local.StartParsing` true))))))

(fn `UserConstructionScript`)