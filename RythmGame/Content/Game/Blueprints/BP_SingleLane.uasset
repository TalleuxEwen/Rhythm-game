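; Single lane of a rhythm game that spawns falling notes at a given BPM and judges hits.
; StartAnimation moves the ring by timeline, then checks bad, sweet and medium overlap zones for BPI_HitObject notes before easing it back.
; Hits update WBP_HUD combo and score with Wwise audio, plus Niagara on good hits; notes reaching the delete zone reset combo.
; Notes entering the medium zone call TriggerMusicPlay.
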(event `self.ReceiveBeginPlay`
  (bind _material (`self.Material`))
  (`/Engine/EditorBlueprintResources/StandardMacros.IsValid` (`self.Material`)
    (:`Is Valid`
      (`PrimitiveComponent.SetMaterial` (`self.Ring`) 0 _material)
      (`PrimitiveComponent.SetMaterial` (`self.StaticMesh1`) 0 _material)
      (`PrimitiveComponent.SetMaterial` (`self.StaticMesh2`) 0 _material)
      (`PrimitiveComponent.SetMaterial` (`self.SphereStart`) 0 _material)
      (`NiagaraComponent.SetVariableMaterial` (`self.NS_NoteTriggerInGame`) "RuntimeMat" _material))))

(event `StartAnimation`
  (`|ExecutionSequence`
    (:`then_0`
      (`/Engine/EditorBlueprintResources/StandardMacros.DoOnce` false
        (:`Completed`
          (set `self.DefaultTransform` (`SceneComponent.GetRelativeTransform` (`self.Ring`))))))
    (:`then_1`
      (bind (_direction _newtrack_0) (`Timeline|Timeline` :!via `PlayFromStart`)
        (:`Update`
          (`SceneComponent.K2_SetRelativeTransform` (`self.Ring`) (`KismetMathLibrary.TLerp` (`self.DefaultTransform`) (`SceneComponent.GetRelativeTransform` (`self.RingAnim`)) _newtrack_0) false false))
        (:`Finished`
          (`self.HitSphereWithCooldown`)
          (`self.EndAnimation`))))))

(event `EndAnimation`
  (bind (_direction _newtrack_0) (`Timeline|Timeline_0` :!via `PlayFromStart`)
    (:`Update`
      (`SceneComponent.K2_SetRelativeTransform` (`self.Ring`) (`KismetMathLibrary.TLerp` (`SceneComponent.GetRelativeTransform` (`self.Ring`)) (`self.DefaultTransform`) _newtrack_0) false false))))

(event `SpawnSphere`
  (params (BPM :type "Float (double-precision)"))
  (bind _returnvalue (`|SpawnActorFromClass` "/Game/Game/Blueprints/BP_FallingNote.BP_FallingNote_C" (`SceneComponent.GetRelativeTransform` (`self.SphereStart`)) "AlwaysSpawn" "MultiplyWithRoot" null null))
  (`self.K2_AttachToActor` _returnvalue self "None" "KeepRelative" "KeepRelative" "KeepRelative" true)
  (`PrimitiveComponent.SetMaterial` (`/Game/Game/Blueprints/BP_FallingNote.Sphere` _returnvalue) 0 (`self.Material`))
  (`/Game/Game/Blueprints/BP_FallingNote.StartFalling` _returnvalue (`SceneComponent.RelativeLocation` (`self.SphereStart`)) (`SceneComponent.RelativeLocation` (`self.SphereEnd`)) (`SceneComponent.RelativeLocation` (`self.SphereFullEnd`)) BPM))

(event `HitSphereWithCooldown`
  (for _array_element (`PrimitiveComponent.GetOverlappingActors` (`self.SphereHitBadSpot`) null)
    (if (`KismetSystemLibrary.DoesImplementInterface` _array_element "/Game/Game/Blueprints/BPI_HitObject.BPI_HitObject_C")
      (message `/Game/Game/Blueprints/BPI_HitObject.Hit` _array_element)
      (`KismetSystemLibrary.PrintString` "bad")
      (`AkGameplayStatics.PostEvent` "/Game/WwiseAudio/Events/Default_Work_Unit/Play_483709__camouflaged_noob__button2.Play_483709__camouflaged_noob__button2")
      (bind _foundwidgets (`WidgetBlueprintLibrary.GetAllWidgetsOfClass` "/Game/Game/Blueprints/Widgets/WBP_HUD.WBP_HUD_C" false))
      (`/Game/Game/Blueprints/Widgets/WBP_HUD.UpdateCombo` (`|GetArrayItem` _foundwidgets) 0 true)))
  (for _array_element_2 (`PrimitiveComponent.GetOverlappingActors` (`self.SphereHitSweetSpot`) null)
    (if (`KismetSystemLibrary.DoesImplementInterface` _array_element_2 "/Game/Game/Blueprints/BPI_HitObject.BPI_HitObject_C")
      (message `/Game/Game/Blueprints/BPI_HitObject.Hit` _array_element_2)
      (`KismetSystemLibrary.PrintString` "sweet")
      (bind _foundwidgets_2 (`WidgetBlueprintLibrary.GetAllWidgetsOfClass` "/Game/Game/Blueprints/Widgets/WBP_HUD.WBP_HUD_C" false))
      (bind _output (`|GetArrayItem` _foundwidgets_2))
      (`/Game/Game/Blueprints/Widgets/WBP_HUD.UpdateCombo` _output 1 false)
      (`/Game/Game/Blueprints/Widgets/WBP_HUD.UpdateScore` _output 50)
      (`ActorComponent.Activate` (`self.NS_NoteTriggerInGame`) false :!label _label)
      (`AkGameplayStatics.PostEvent` "/Game/WwiseAudio/Events/Default_Work_Unit/Play_318968__djm62__successarpeggio.Play_318968__djm62__successarpeggio")))
  (for _array_element_3 (`PrimitiveComponent.GetOverlappingActors` (`self.SphereHitMediumSpot`) null)
    (if (`KismetSystemLibrary.DoesImplementInterface` _array_element_3 "/Game/Game/Blueprints/BPI_HitObject.BPI_HitObject_C")
      (message `/Game/Game/Blueprints/BPI_HitObject.Hit` _array_element_3)
      (`KismetSystemLibrary.PrintString` "medium")
      (bind _foundwidgets_3 (`WidgetBlueprintLibrary.GetAllWidgetsOfClass` "/Game/Game/Blueprints/Widgets/WBP_HUD.WBP_HUD_C" false))
      (bind _output_2 (`|GetArrayItem` _foundwidgets_3))
      (`/Game/Game/Blueprints/Widgets/WBP_HUD.UpdateCombo` _output_2 1 false)
      (`/Game/Game/Blueprints/Widgets/WBP_HUD.UpdateScore` _output_2 10)
      (goto _label))))

(event `self.SphereDeleteZone.OnComponentBeginOverlap`
  (params (OverlappedComponent :type "PrimitiveComponent Object Reference") (OtherActor :type "Actor Object Reference") (OtherComp :type "PrimitiveComponent Object Reference") (OtherBodyIndex :type Integer) (bFromSweep :type Boolean) (SweepResult :type "HitResult Structure (by ref)"))
  (message `/Game/Game/Blueprints/BPI_HitObject.Hit` OtherActor)
  (bind _foundwidgets (`WidgetBlueprintLibrary.GetAllWidgetsOfClass` "/Game/Game/Blueprints/Widgets/WBP_HUD.WBP_HUD_C" false))
  (`/Game/Game/Blueprints/Widgets/WBP_HUD.UpdateCombo` (`|GetArrayItem` _foundwidgets) 0 true))

(event `self.SphereHitMediumSpot.OnComponentBeginOverlap`
  (params (OverlappedComponent :type "PrimitiveComponent Object Reference") (OtherActor :type "Actor Object Reference") (OtherComp :type "PrimitiveComponent Object Reference") (OtherBodyIndex :type Integer) (bFromSweep :type Boolean) (SweepResult :type "HitResult Structure (by ref)"))
  (if (`KismetSystemLibrary.DoesImplementInterface` OtherActor "/Game/Game/Blueprints/BPI_HitObject.BPI_HitObject_C")
    (`self.TriggerMusicPlay`)))

(fn `UserConstructionScript`)