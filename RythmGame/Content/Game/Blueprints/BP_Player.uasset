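; BP_Player is the player Blueprint that takes lane key input, with six lanes in total.
; On BeginPlay it adds the IMC_PlayerIngame Enhanced Input mapping context to its player controller's subsystem.
; Each of the six lane input actions forwards its lane number to CallKeyPress, whose logic is not defined in these graphs.
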(event `self.ReceiveBeginPlay`
  (bind _asplayer_controller (cast `PlayerController` (`self.GetController`)))
  (`EnhancedInputSubsystemInterface.AddMappingContext` (pcsubsystem `EnhancedInputLocalPlayerSubsystem` _asplayer_controller) "/Game/Game/Inputs/IMC_PlayerIngame.IMC_PlayerIngame" 0 (struct)))

(event `EnhancedInput|/Game/Game/Inputs/IA/IA_LaneKeyPress1`
  (params (ActionValue :type Boolean) (ElapsedSeconds :type "Float (double-precision)") (TriggeredSeconds :type "Float (double-precision)") (InputAction :type "InputAction Object Reference" :default "/Game/Game/Inputs/IA/IA_LaneKeyPress1.IA_LaneKeyPress1"))
  (:`Triggered`
    (`self.KeyPress` 1)))

(event `EnhancedInput|/Game/Game/Inputs/IA/IA_LaneKeyPress2`
  (params (ActionValue :type Boolean) (ElapsedSeconds :type "Float (double-precision)") (TriggeredSeconds :type "Float (double-precision)") (InputAction :type "InputAction Object Reference" :default "/Game/Game/Inputs/IA/IA_LaneKeyPress2.IA_LaneKeyPress2"))
  (:`Triggered`
    (`self.KeyPress` 2)))

(event `EnhancedInput|/Game/Game/Inputs/IA/IA_LaneKeyPress3`
  (params (ActionValue :type Boolean) (ElapsedSeconds :type "Float (double-precision)") (TriggeredSeconds :type "Float (double-precision)") (InputAction :type "InputAction Object Reference" :default "/Game/Game/Inputs/IA/IA_LaneKeyPress3.IA_LaneKeyPress3"))
  (:`Triggered`
    (`self.KeyPress` 3)))

(event `EnhancedInput|/Game/Game/Inputs/IA/IA_LaneKeyPress4`
  (params (ActionValue :type Boolean) (ElapsedSeconds :type "Float (double-precision)") (TriggeredSeconds :type "Float (double-precision)") (InputAction :type "InputAction Object Reference" :default "/Game/Game/Inputs/IA/IA_LaneKeyPress4.IA_LaneKeyPress4"))
  (:`Triggered`
    (`self.KeyPress` 4)))

(event `EnhancedInput|/Game/Game/Inputs/IA/IA_LaneKeyPress5`
  (params (ActionValue :type Boolean) (ElapsedSeconds :type "Float (double-precision)") (TriggeredSeconds :type "Float (double-precision)") (InputAction :type "InputAction Object Reference" :default "/Game/Game/Inputs/IA/IA_LaneKeyPress5.IA_LaneKeyPress5"))
  (:`Triggered`
    (`self.KeyPress` 5)))

(event `EnhancedInput|/Game/Game/Inputs/IA/IA_LaneKeyPress6`
  (params (ActionValue :type Boolean) (ElapsedSeconds :type "Float (double-precision)") (TriggeredSeconds :type "Float (double-precision)") (InputAction :type "InputAction Object Reference" :default "/Game/Game/Inputs/IA/IA_LaneKeyPress6.IA_LaneKeyPress6"))
  (:`Triggered`
    (`self.KeyPress` 6)))

(fn `UserConstructionScript`)